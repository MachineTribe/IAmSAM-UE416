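; GameMode Blueprint that acts as a central event relay for UI actions and audio settings.
; Custom events for text commit, options and login clicks, and conversation changes each call a matching event, apparently an event dispatcher.
; Volume and FX volume events store the new value before broadcasting, and two getters expose the stored values.
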(event Custom|Ev_TextCommited
  (Default|CallEventTextCommitted))

(event Custom|EV_SetFXVolume
  (params (volume :type Float%20%28single-precision%29))
  (Variables|Default|SetcurrentFXVolume volume)
  (Default|CallEventSetFXVolume))

(event Custom|EV_OptionsClicked
  (Default|CallEventOptionsClicked))

(event Custom|EV_LoginClicked
  (Default|CallEventLoginClicked))

(event Custom|EV_ConversationChanged
  (Default|CallEventConversationChanged))

(event Custom|EV_SetVolume
  (params (volume :type Float%20%28single-precision%29))
  (Variables|Default|SetcurrentVolume volume)
  (Default|CallEventSetVolume))

(event EventBeginPlay)

(fn ConstructionScript)

(fn GetCurrentVolume
  (return (Variables|Default|GetcurrentVolume)))

(fn GetFXVolume
  (return (Variables|Default|GetcurrentFXVolume)))